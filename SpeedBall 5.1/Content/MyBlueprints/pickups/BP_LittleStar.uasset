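; BP_LittleStar is a collectible star pickup that bobs and rotates in place from a timeline started on BeginPlay.
; Any overlap with its sphere, with no check on the other actor, calls AddStar on the game mode through what appear to be interface messages.
; A second timeline then lifts the actor by adding its curve value to the current height each update, and destroys it when finished.
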(event OnComponentBeginOverlap(Sphere)
  (params (OverlappedComponent :type Primitive%20Component%20Object%20Reference) (OtherActor :type Actor%20Object%20Reference) (OtherComp :type Primitive%20Component%20Object%20Reference) (OtherBodyIndex :type Integer) (bFromSweep :type Boolean) (SweepResult :type Hit%20Result%20Structure%20%28by%20ref%29))
  (bind _gamemode (Class|IGameMode|GetGameModeRef(Message) (Game|GetGameMode)))
  (Class|IGameMode|AddStar(Message) _gamemode)
  (CallFunction|StarLooted))

(event Custom|StarLooted
  (bind _returnvalue (Transformation|GetActorLocation))
  (bind _flyup (Timeline|StarLootMovement Play)
    (:Update
      (Transformation|SetActorRelativeLocation (Math|Vector|MakeVector (.x _returnvalue) (.y _returnvalue) (+ (.z _returnvalue) (.z _flyup)))))
    (:Finished
      (Actor|DestroyActor))))

(event EventBeginPlay
  (bind (_direction _zlocation _zrotation) (Timeline|anim_wobbleupdown Play)
    (:Update
      (Transformation|SetRelativeLocationAndRotation (Variables|Default|GetLittleStar) (Math|Vector|MakeVector 0.0 0.0 (.z _zlocation)) (Math|Rotator|MakeRotator 0.0 0.0 (.z _zrotation)) false false))))

(event Collision|EventActorBeginOverlap
  (params (OtherActor :type Actor%20Object%20Reference)))

(event EventTick
  (params (DeltaSeconds :type Float%20%28single-precision%29)))

(fn ConstructionScript)